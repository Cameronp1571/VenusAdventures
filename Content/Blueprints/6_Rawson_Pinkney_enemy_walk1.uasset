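; Paper2D walking enemy actor that patrols between PointA and PointB via InterpToMovement control points set in construction, but self-destructs 1.5 seconds after spawning.
; On alternate movement reversals the flipbook is set to a fixed rotation; the reset rotation is unwired.
; Overlaps with its own class destroy both actors, while sprite overlaps add upward force and call ApplyDamage without a target.
; The custom Damage function and Damage_2 event are empty stubs.
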(event OnInterptoReverse(InterpToMovement)
  (params (ImpactResult :type Hit%20Result%20Structure%20%28by%20ref%29) (Time :type Float%20%28single-precision%29))
  ;[1 1 1] Projectile
  (Utilities|FlowControl|FlipFlop
    (:A
      (Transformation|SetWorldRotation (Variables|Default|GetPaperFlipbook) "0,180.000000,0.000000" false false))))

(event OnComponentBeginOverlap(Sprite)
  (params (OverlappedComponent :type Primitive%20Component%20Object%20Reference) (OtherActor :type Actor%20Object%20Reference) (OtherComp :type Primitive%20Component%20Object%20Reference) (OtherBodyIndex :type Integer) (bFromSweep :type Boolean) (SweepResult :type Hit%20Result%20Structure%20%28by%20ref%29))
  ;[1 1 1] Projectile
  (Utilities|Casting|CastTo6_Rawson_Pinkney_enemy_walk1 OtherActor)
  (Class|PrimitiveComponent|AddForceatLocation (Variables|Default|GetPaperFlipbook) "0.000000, 0,500.000000" "0, 0, 0" "None")
  (Game|Damage|ApplyDamage 0 (* (.x (.Normal (Collision|BreakHitResult SweepResult))) -4e+02) 0 0 "/Engine/EngineDamageTypes/DmgTypeBP_Environmental.DmgTypeBP_Environmental_C"))

(event Custom|Damage_2
  (params (Damage_out :type Integer)))

(event EventBeginPlay
  (Utilities|FlowControl|Delay 1.5)
  (Actor|DestroyActor))

(event EventTick
  (params (DeltaSeconds :type Float%20%28single-precision%29)))

(event Collision|EventActorBeginOverlap
  (params (OtherActor :type Actor%20Object%20Reference))
  (Utilities|FlowControl|Sequence
    (:then_0
      (bind _as6_rawson_pinkney_enemy_walk_1 (Utilities|Casting|CastTo6_Rawson_Pinkney_enemy_walk1 OtherActor))
      (Actor|DestroyActor _as6_rawson_pinkney_enemy_walk_1))
    (:then_1
      (bind _as6_rawson_pinkney_enemy_walk_1_2 (Utilities|Casting|CastTo6_Rawson_Pinkney_enemy_walk1 OtherActor))
      (CallFunction|Damage _as6_rawson_pinkney_enemy_walk_1_2)
      (Actor|DestroyActor)
      (Development|PrintString "hit"))))

(fn ConstructionScript
  (Variables|/Script/Engine.InterpToMovementComponent|SetControlPoints (Variables|Default|GetInterpToMovement) (Utilities|Array|MakeArray (Utilities|Struct|MakeInterpControlPoint (Variables|Default|Getpoint%20b) true) (Utilities|Struct|MakeInterpControlPoint (Variables|Default|Getpoint%20a) true))))

(fn Damage
  (params (Damage_in :type Integer)))