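; Walking 2D Paper2D enemy that patrols between PointA and PointB.
; The construction script feeds both points as relative control points into InterpToMovement; on reverse, a FlipFlop rotates the flipbook 180 degrees every other time, with the rotation back left unwired.
; Sprite overlap with another instance of this class pushes the flipbook upward and calls ApplyDamage scaled by the hit normal's X, with no target set.
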(event OnInterptoReverse(InterpToMovement)
  (params (ImpactResult :type Hit%20Result%20Structure%20%28by%20ref%29) (Time :type Float%20%28single-precision%29))
  ;[1 1 1] Projectile
  (Utilities|FlowControl|FlipFlop
    (:A
      (Transformation|SetWorldRotation (Variables|Default|GetPaperFlipbook) "0,180.000000,0.000000" false false))))

(event OnComponentBeginOverlap(Sprite)
  (params (OverlappedComponent :type Primitive%20Component%20Object%20Reference) (OtherActor :type Actor%20Object%20Reference) (OtherComp :type Primitive%20Component%20Object%20Reference) (OtherBodyIndex :type Integer) (bFromSweep :type Boolean) (SweepResult :type Hit%20Result%20Structure%20%28by%20ref%29))
  ;[1 1 1] Projectile
  (Utilities|Casting|CastTo6_Rawson_Pinkney_enemy_walk1 OtherActor)
  (Class|PrimitiveComponent|AddForceatLocation (Variables|Default|GetPaperFlipbook) "0.000000, 0,500.000000" "0, 0, 0" "None")
  (Game|Damage|ApplyDamage 0 (* (.x (.Normal (Collision|BreakHitResult SweepResult))) -4e+02) 0 0 "/Script/Engine.DamageType"))

(event Collision|EventActorBeginOverlap
  (params (OtherActor :type Actor%20Object%20Reference)))

(event EventTick
  (params (DeltaSeconds :type Float%20%28single-precision%29)))

(fn ConstructionScript
  (Variables|/Script/Engine.InterpToMovementComponent|SetControlPoints (Variables|Default|GetInterpToMovement) (Utilities|Array|MakeArray (Utilities|Struct|MakeInterpControlPoint (Variables|Default|Getpoint%20b) true) (Utilities|Struct|MakeInterpControlPoint (Variables|Default|Getpoint%20a) true))))